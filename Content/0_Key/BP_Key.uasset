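; BP_Key is a key pickup the player grabs through its GrabComponent.
; On grab it plays a pickup sound at the key mesh and sets IsTaken.
; A proximity highlight using custom depth, meant to show on an untaken key within range of the player, is present but unconnected, so it never runs.
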(event `self.ReceiveTick`
  (params (DeltaSeconds :type "Float (single-precision)")))

(event `self.GrabComponent.OnGrabbed`
  (`GameplayStatics.PlaySoundAtLocation` "/Game/sounds/keypickup.keypickup" (`SceneComponent.K2_GetComponentLocation` (`self.Key`)) (struct) 1.0 1.0 0.0 null null null)
  (if (not (`self.isTaken`))
    (set `self.isTaken` true)))

(fn `UserConstructionScript`)